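; Visualization Blueprint that leaves a trail of markers tracing a point offset from its Mesh along that mesh's up vector.
; A looping quarter-second timer started on BeginPlay samples the Mesh's world location plus its up vector scaled by Dist.
; Each sample becomes a new instance on the Points component, so markers accumulate without spawning actors and are never cleared here.
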(event `self.ReceiveBeginPlay`
  (`KismetSystemLibrary.K2_SetTimerDelegate` (delegate `MarkLocation`) 0.25 true))

(event `MarkLocation`
  (bind _mesh (`self.Mesh`))
  (`InstancedStaticMeshComponent.AddInstance` (`self.Points`) (`KismetMathLibrary.Conv_VectorToTransform` (+ (* (`SceneComponent.GetUpVector` _mesh) (`self.Dist`)) (`SceneComponent.K2_GetComponentLocation` _mesh)))))

(fn `UserConstructionScript`)